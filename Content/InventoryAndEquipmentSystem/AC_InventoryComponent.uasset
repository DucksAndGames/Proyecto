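; Inventory actor component that stores picked-up items as a class array and shows or hides the inventory UI.
; Showing creates a WB_Inventory widget for the local player controller and fills it from the array; hiding removes it from the viewport.
; Adding an item records its class, then plays either a local 2D sound or, if replication is enabled, a sound at the item's mesh through server and multicast events.
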(event Custom|Server_PlaySound
  (params (Sound :type Sound%20Base%20Object%20Reference) (Location :type Vector))
  (CallFunction|MCPlaySound Sound Location))

(event Custom|MC_PlaySound
  (params (Sound :type Sound%20Base%20Object%20Reference) (Location :type Vector))
  (Audio|PlaySoundatLocation Sound Location "0, 0, 0" 1.0 1.0 0.0 0 0 0 0))

(event EventBeginPlay)

(event EventTick
  (params (DeltaSeconds :type Float%20%28single-precision%29)))

(fn FShowInventory
  (bind _returnvalue (Game|GetPlayerController 0))
  ;[1 1 1] Es el personaje poseido
  (if (Pawn|IsLocalPlayerController _returnvalue)
    (bind _returnvalue_2 (UserInterface|CreateWidget "/Game/InventoryAndEquipmentSystem/Widgets/WB_Inventory.WB_Inventory_C" _returnvalue))
    (bind _output_get (Variables|Default|SetWB_Inventery _returnvalue_2))
    (UserInterface|Viewport|AddtoViewport _output_get 0)
    (Default|FUpdate _returnvalue_2 (Variables|Default|GetInventory))))

(fn FHideInventory
  (bind _wb_inventery (Variables|Default|GetWB_Inventery))
  (Utilities|IsValid _wb_inventery
    (:Is%20Valid
      (Widget|RemovefromParent _wb_inventery))))

(fn FAddItemInventory
  (params (NewItem :type BP%20Master%20Item%20Object%20Reference%20%28by%20ref%29))
  (bind _staticmesh (Variables|/Game/InventoryAndEquipmentSystem/BP_MasterItem.BP_MasterItem_C|GetStaticMesh NewItem))
  (bind _returnvalue (Transformation|GetWorldLocation _staticmesh))
  (Utilities|Array|Add (Variables|Default|GetInventory) (Utilities|GetClass NewItem))
  (if (Variables|Default|GetReplicatePickupSound?)
    (Networking|SwitchHasAuthority
      (:Authority
        (CallFunction|MCPlaySound 0 _returnvalue))
      (:Remote
        (CallFunction|ServerPlaySound 0 _returnvalue)))
    (else
      (Audio|PlaySound2D 0 1.0 1.0 0.0 0 0))))