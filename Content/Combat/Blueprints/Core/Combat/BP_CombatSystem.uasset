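; Combat system Blueprint that tracks the units in combat and keeps their placement in sync with the tile grid.
; Adding, removing or moving a unit updates tile occupancy and teleports its actor to the tile, using a sentinel index for off-grid.
; It binds to grid generation and tile update events, re-placing affected units or destroying those left on unwalkable tiles.
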(event EventBeginPlay
  (bind _grid (Variables|Default|GetGrid))
  (EventDispatchers|BindEventtoOnGridGenerated _grid (EventDispatchers|CreateEvent :!event OnGridGenerated))
  (EventDispatchers|BindEventtoOnTileDataUpdated _grid (EventDispatchers|CreateEvent :!event OnTileDataUpdated)))

(event Collision|EventActorBeginOverlap
  (params (OtherActor :type Actor%20Object%20Reference)))

(event EventTick
  (params (DeltaSeconds :type Float%20%28single-precision%29)))

(fn ConstructionScript)

(fn AddUnitinCombat
  (params (Unit :type BP%20Unit%20Object%20Reference) (Index :type Int%20Point%20Structure))
  (Utilities|Array|Add (Variables|Default|GetUnitsInCombat) Unit)
  (CallFunction|SetUnitIndexonGrid Unit Index))

(fn RemoveUnitfromCombat
  (params (Unit :type BP%20Unit%20Object%20Reference) (DestroyUnit :type Boolean))
  (Utilities|Array|RemoveItem (Variables|Default|GetUnitsInCombat) Unit)
  (CallFunction|SetUnitIndexonGrid Unit (Utilities|Struct|MakeIntPoint -999 -999))
  (if DestroyUnit
    (Actor|DestroyActor Unit)))

(fn SetUnitIndexonGrid
  (params (Unit :type BP%20Unit%20Object%20Reference) (Index :type Int%20Point%20Structure))
  (Utilities|FlowControl|Sequence
    (:then_0
      (if (!= (Variables|/Game/Combat/Blueprints/Core/Units/BP_Unit.BP_Unit_C|GetIndex Unit) Index)
        (Utilities|FlowControl|Sequence
          (:then_0
            (bind _output_get (LocalVariables|SetPreviousTile (.Value (Utilities|Map|Find (Variables|/Game/Combat/Blueprints/Core/Grid/BP_Grid.BP_Grid_C|GetGridTiles (Variables|Default|GetGrid)) (Variables|/Game/Combat/Blueprints/Core/Units/BP_Unit.BP_Unit_C|GetIndex Unit)))))
            (if (== (Utilities|Struct|BreakS_TileData _output_get) Unit)
              (bind _structout (Utilities|Struct|SetmembersinS_TileData (LocalVariables|GetPreviousTile)))
              (Utilities|Map|Add (Variables|/Game/Combat/Blueprints/Core/Grid/BP_Grid.BP_Grid_C|GetGridTiles (Variables|Default|GetGrid)) (Utilities|Struct|BreakS_TileData _structout) _structout)))
          (:then_1
            (Variables|/Game/Combat/Blueprints/Core/Units/BP_Unit.BP_Unit_C|SetIndex Unit Index)
            (if (!= Index (Utilities|Struct|MakeIntPoint -999 -999))
              (bind _structout_2 (Utilities|Struct|SetmembersinS_TileData (.Value (Utilities|Map|Find (Variables|/Game/Combat/Blueprints/Core/Grid/BP_Grid.BP_Grid_C|GetGridTiles (Variables|Default|GetGrid)) Index)) Unit))
              (Utilities|Map|Add (Variables|/Game/Combat/Blueprints/Core/Grid/BP_Grid.BP_Grid_C|GetGridTiles (Variables|Default|GetGrid)) (Utilities|Struct|BreakS_TileData _structout_2) _structout_2))))))
    (:then_1
      (Transformation|SetActorLocation Unit (select (.ReturnValue (Utilities|Map|Find (Variables|/Game/Combat/Blueprints/Core/Grid/BP_Grid.BP_Grid_C|GetGridTiles (Variables|Default|GetGrid)) Index)) (.location (Utilities|Struct|BreakS_TileData (.Value (Utilities|Map|Find (Variables|/Game/Combat/Blueprints/Core/Grid/BP_Grid.BP_Grid_C|GetGridTiles (Variables|Default|GetGrid)) Index)))) "-999999.000000,-99999.000000,-99999.000000") false false))))

(fn OnGridGenerated
  (bind _output_get (LocalVariables|SetCopyOfUnitsInCombat (Variables|Default|GetUnitsInCombat)))
  (for _array_element _output_get
    (if (Default|IsTileWalkable (Variables|Default|GetGrid) (Variables|/Game/Combat/Blueprints/Core/Units/BP_Unit.BP_Unit_C|GetIndex _array_element))
      (CallFunction|SetUnitIndexonGrid _array_element (Variables|/Game/Combat/Blueprints/Core/Units/BP_Unit.BP_Unit_C|GetIndex _array_element))
      (else
        (CallFunction|RemoveUnitfromCombat _array_element true)))))

(fn OnTileDataUpdated
  (params (index :type Int%20Point%20Structure))
  (bind _output_get (LocalVariables|SetCopyOfUnitsInCombat (Variables|Default|GetUnitsInCombat)))
  (bind _array_element (Utilities|Array|ForEachLoopwithBreak _output_get :!label _label)
    (:LoopBody
      (if (Class|KismetMathLibrary|EqualIntPointIntPoint index (Variables|/Game/Combat/Blueprints/Core/Units/BP_Unit.BP_Unit_C|GetIndex _array_element))
        (if (Default|IsTileWalkable (Variables|Default|GetGrid) (Variables|/Game/Combat/Blueprints/Core/Units/BP_Unit.BP_Unit_C|GetIndex _array_element))
          (CallFunction|SetUnitIndexonGrid _array_element (Variables|/Game/Combat/Blueprints/Core/Units/BP_Unit.BP_Unit_C|GetIndex _array_element))
          (goto _label Break)
          (else
            (CallFunction|RemoveUnitfromCombat _array_element true)
            (goto _label Break)))))))