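; Grid pathfinder that runs A* between two walkable tiles of a hexagonal combat grid and returns the tile path.
; Neighbors use doubled-row hex offsets, filtered by walkable type and height step; the diagonals option has no effect.
; A cost-sorted open list feeds expansion until the target is discovered, then previous-index links are walked back to build the path.
; Dispatchers broadcast when pathfinding data is updated or cleared.
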(event EventBeginPlay)

(event Collision|EventActorBeginOverlap
  (params (OtherActor :type Actor%20Object%20Reference)))

(event EventTick
  (params (DeltaSeconds :type Float%20%28single-precision%29)))

(fn ConstructionScript)

(fn GetValidTileNeighbors
  (params (Index :type Int%20Point%20Structure) (IncludeDiagonals :type Boolean))
  ;[1 1 1] To compare the height later
  (LocalVariables|SetInputData (.Value (Utilities|Map|Find (Variables|/Game/Combat/Blueprints/Core/Grid/BP_Grid.BP_Grid_C|GetGridTiles (Variables|Default|GetGrid)) Index)))
  ;[1 1 1] Loop trough all the potential neighbors to validate them+
  (bind _neighbors (Neighbors|GetNeighborsIndexes Index IncludeDiagonals))
  (for _array_element _neighbors
    (LocalVariables|SetData (.Value (Utilities|Map|Find (Variables|/Game/Combat/Blueprints/Core/Grid/BP_Grid.BP_Grid_C|GetGridTiles (Variables|Default|GetGrid)) _array_element)))
    (if (CallFunction|IsTileTypeWallkable (.type (LocalVariables|GetData)))
      (if (<= (Math|Float|Absolute(Float) (- (.z (.location (.transform (LocalVariables|GetData)))) (.z (.location (.transform (LocalVariables|GetInputData)))))) (.z (Variables|/Game/Combat/Blueprints/Core/Grid/BP_Grid.BP_Grid_C|GetGridTile%20Size (Variables|Default|GetGrid))))
        ;[1 1 1] Valid Neighbors
        (Utilities|Array|Add (LocalVariables|GetRet) (Utilities|Struct|MakeS_PathfindingData (.index (LocalVariables|GetData)) 1 999999 999999 Index)))))
  (return (LocalVariables|GetRet)))

(fn GetNeighborsIndexesforHexagon
  (params (Index :type Int%20Point%20Structure))
  (return (Utilities|Array|MakeArray (+ Index (Utilities|Struct|MakeIntPoint 1 1)) (+ Index (Utilities|Struct|MakeIntPoint 0 2)) (+ Index (Utilities|Struct|MakeIntPoint -1 1)) (+ Index (Utilities|Struct|MakeIntPoint -1 -1)) (+ Index (Utilities|Struct|MakeIntPoint 0 -2)) (+ Index (Utilities|Struct|MakeIntPoint 1 -1)))))

(fn GetNeighborsIndexes
  (params (Index :type Int%20Point%20Structure) (IncludeDiagonals :type Boolean))
  (return (Neighbors|GetNeighborsIndexesforHexagon Index)))

(fn FindPath
  (params (Start :type Int%20Point%20Structure) (Target :type Int%20Point%20Structure) (Diagonals :type Boolean))
  (Variables|Default|SetIncludeDiagonals Diagonals)
  (Variables|Default|SetStartIndex Start)
  (Variables|Default|SetTargetIndex Target)
  (CallFunction|ClearGeneratedData)
  ;[1 1 1] Check if variables are valid
  (bind _isvalid (CallFunction|IsInputDataValid))
  (if _isvalid
    (CallFunction|DiscoverTile (Utilities|Struct|MakeS_PathfindingData (Variables|Default|GetStartIndex) 1 0 (CallFunction|GetMinimumCostBetweenTwoTiles (Variables|Default|GetStartIndex) (Variables|Default|GetTargetIndex) (Variables|Default|GetIncludeDiagonals)) "(X=-999,Y=-999)"))
    (while (> (Utilities|Array|Length (Variables|Default|GetDiscoveredTileIndexes)) 0)
      (bind _foundtargettile (CallFunction|AnalyseNextDiscoveredTile))
      (if _foundtargettile
        (bind _path (CallFunction|GeneratePath))
        (for _array_element _path
          (return _path))))
    (return (Utilities|Array|MakeArray ""))
    (else
      (return (Utilities|Array|MakeArray "")))))

(fn IsInputDataValid
  (if (!= (Variables|Default|GetTargetIndex) (Variables|Default|GetStartIndex))
    (if (Default|IsTileWalkable (Variables|Default|GetGrid) (Variables|Default|GetStartIndex))
      (if (Default|IsTileWalkable (Variables|Default|GetGrid) (Variables|Default|GetTargetIndex))
        (return true)
        (else
          (return false)))
      (else
        (return false)))
    (else
      (return false))))

(fn DiscoverTile
  (params (TilePathData :type S%20Pathfinding%20Data%20Structure))
  (bind _index (Utilities|Struct|BreakS_PathfindingData TilePathData))
  (Utilities|Map|Add (Variables|Default|GetPatfindingData) _index TilePathData)
  (CallFunction|InsertTileinDiscoveredArray TilePathData)
  (Default|CallOnPathfindingDataUpdated _index))

(fn GetMinimumCostBetweenTwoTiles
  (params (Index1 :type Int%20Point%20Structure) (Index2 :type Int%20Point%20Structure) (Diagonals :type Boolean))
  (bind _returnvalue (- Index1 Index2))
  (bind _returnvalue_2 (Math|Integer|Absolute(Integer) (.x _returnvalue)))
  (return (+ _returnvalue_2 (Math|Integer|Max(Integer) (/ (- (Math|Integer|Absolute(Integer) (.y _returnvalue)) _returnvalue_2) 2)))))

(fn AnalyseNextDiscoveredTile
  (bind _tilepathdata (CallFunction|PullCheapestTileOutOfDiscoveredList))
  (Variables|Default|SetCurrentDiscoveredTile _tilepathdata)
  (bind _neighbors (Neighbors|GetValidTileNeighbors (.Index (Utilities|Struct|BreakS_PathfindingData (Variables|Default|GetCurrentDiscoveredTile))) (Variables|Default|GetIncludeDiagonals)))
  (Variables|Default|SetCurrentsNeighbors _neighbors)
  (while (> (Utilities|Array|Length (Variables|Default|GetCurrentsNeighbors)) 0)
    (bind _istargettile (CallFunction|DiscoverNextNeighbor))
    (if _istargettile
      (return true)))
  (return false))

(fn GeneratePath
  (LocalVariables|SetCurrent (Variables|Default|GetTargetIndex))
  (while (!= (LocalVariables|GetCurrent) (Variables|Default|GetStartIndex))
    (Utilities|Array|Add (LocalVariables|GetInvertedPath) (LocalVariables|GetCurrent))
    (LocalVariables|SetCurrent (.PreviousIndex (Utilities|Struct|BreakS_PathfindingData (.Value (Utilities|Map|Find (Variables|Default|GetPatfindingData) (LocalVariables|GetCurrent)))))))
  (bind _arrayelement (Utilities|Array|ReverseforEachLoop (LocalVariables|GetInvertedPath))
    (:LoopBody
      (Utilities|Array|Add (LocalVariables|GetRet) _arrayelement))
    (:Completed
      (return (LocalVariables|GetRet)))))

(fn PullCheapestTileOutOfDiscoveredList
  (LocalVariables|SetTileIndex (Utilities|Array|Get(acopy) (Variables|Default|GetDiscoveredTileIndexes)))
  (Utilities|Array|RemoveIndex (Variables|Default|GetDiscoveredTileSortingCosts))
  (Utilities|Array|RemoveIndex (Variables|Default|GetDiscoveredTileIndexes))
  (Utilities|Array|Add (Variables|Default|GetAnalysedTileIndexes) (LocalVariables|GetTileIndex))
  (return (.Value (Utilities|Map|Find (Variables|Default|GetPatfindingData) (LocalVariables|GetTileIndex)))))

(fn DiscoverNextNeighbor
  (Variables|Default|SetCurrentNeighbor (Utilities|Array|Get(acopy) (Variables|Default|GetCurrentsNeighbors)))
  (Utilities|Array|RemoveIndex (Variables|Default|GetCurrentsNeighbors))
  (if (not (Utilities|Array|ContainsItem (Variables|Default|GetAnalysedTileIndexes) (.Index (Utilities|Struct|BreakS_PathfindingData (Variables|Default|GetCurrentNeighbor)))))
    (LocalVariables|SetCostFromStart (+ (.CostFromStart (Utilities|Struct|BreakS_PathfindingData (Variables|Default|GetCurrentDiscoveredTile))) (.CostToEnterTile (Utilities|Struct|BreakS_PathfindingData (Variables|Default|GetCurrentNeighbor)))))
    (bind _output_get (LocalVariables|SetIndexInDiscovered (Utilities|Array|FindItem (Variables|Default|GetDiscoveredTileIndexes) (.Index (Utilities|Struct|BreakS_PathfindingData (Variables|Default|GetCurrentNeighbor))))))
    (if (== _output_get -1)
      _
      (else
        (bind _output_get_2 (Variables|Default|SetCurrentNeighbor (.Value (Utilities|Map|Find (Variables|Default|GetPatfindingData) (.Index (Utilities|Struct|BreakS_PathfindingData (Variables|Default|GetCurrentNeighbor)))))))
        (if (< (LocalVariables|GetCostFromStart) (.CostFromStart (Utilities|Struct|BreakS_PathfindingData _output_get_2)))
          (Utilities|Array|RemoveIndex (Variables|Default|GetDiscoveredTileIndexes) (LocalVariables|GetIndexInDiscovered))
          (Utilities|Array|RemoveIndex (Variables|Default|GetDiscoveredTileSortingCosts) (LocalVariables|GetIndexInDiscovered))
          (else
            (return false)))))
    (CallFunction|DiscoverTile (Utilities|Struct|MakeS_PathfindingData (.index (Variables|Default|GetCurrentNeighbor)) (.costtoentertile (Variables|Default|GetCurrentNeighbor)) (LocalVariables|GetCostFromStart) (CallFunction|GetMinimumCostBetweenTwoTiles (.Index (Utilities|Struct|BreakS_PathfindingData (Variables|Default|GetCurrentNeighbor))) (Variables|Default|GetTargetIndex) (Variables|Default|GetIncludeDiagonals)) (.Index (Utilities|Struct|BreakS_PathfindingData (Variables|Default|GetCurrentDiscoveredTile)))))
    (if (Class|KismetMathLibrary|EqualIntPointIntPoint (.Index (Utilities|Struct|BreakS_PathfindingData (Variables|Default|GetCurrentNeighbor))) (Variables|Default|GetTargetIndex))
      (return true)
      (else
        (return false)))
    (else
      (return false))))

(fn InsertTileinDiscoveredArray
  (params (Tiledata :type S%20Pathfinding%20Data%20Structure))
  (bind _discoveredtilesortingcosts (Variables|Default|GetDiscoveredTileSortingCosts))
  (LocalVariables|SetSortingCost (CallFunction|GetTileSortingCost Tiledata))
  (if (== (Utilities|Array|Length (Variables|Default|GetDiscoveredTileSortingCosts)) 0)
    (Utilities|Array|Add (Variables|Default|GetDiscoveredTileSortingCosts) (LocalVariables|GetSortingCost) :!label _label)
    (Utilities|Array|Add (Variables|Default|GetDiscoveredTileIndexes) (.Index (Utilities|Struct|BreakS_PathfindingData Tiledata)))
    (elif (>= (LocalVariables|GetSortingCost) (Utilities|Array|Get(acopy) _discoveredtilesortingcosts (Utilities|Array|LastIndex _discoveredtilesortingcosts)))
      (goto _label)
      (else
        (bind (_array_element _array_index) (Utilities|Array|ForEachLoopwithBreak (Variables|Default|GetDiscoveredTileSortingCosts) :!label _label_2)
          (:LoopBody
            (if (>= _array_element (LocalVariables|GetSortingCost))
              (Utilities|Array|Insert (Variables|Default|GetDiscoveredTileSortingCosts) (LocalVariables|GetSortingCost) _array_index)
              (Utilities|Array|Insert (Variables|Default|GetDiscoveredTileIndexes) (.index Tiledata) _array_index)
              (goto _label_2 Break))))))))

(fn ClearGeneratedData
  (Utilities|Map|Clear (Variables|Default|GetPatfindingData))
  (Utilities|Array|Clear (Variables|Default|GetDiscoveredTileSortingCosts))
  (Utilities|Array|Clear (Variables|Default|GetDiscoveredTileIndexes))
  (Utilities|Array|Clear (Variables|Default|GetAnalysedTileIndexes))
  (Default|CallOnPathfindingDataCleared))

(fn IsDiagonal
  (params (Index%201 :type Int%20Point%20Structure) (Index2 :type Int%20Point%20Structure))
  (bind _neighbors (Neighbors|GetNeighborsIndexes Index%201 false))
  (return (not (Utilities|Array|ContainsItem _neighbors Index2))))

(fn GetTileSortingCost
  (params (TileData :type S%20Pathfinding%20Data%20Structure%20%28by%20ref%29))
  (bind (_index _costtoentertile _costfromstart _minimumcosttotarget) (Utilities|Struct|BreakS_PathfindingData TileData))
  (bind (_index_2 _costtoentertile_2 _costfromstart_2 _minimumcosttotarget_2 _previousindex) (Utilities|Struct|BreakS_PathfindingData TileData))
  (return (+ (* (+ _costfromstart _minimumcosttotarget) 2) (Math|Conversions|ToInteger(Boolean) (CallFunction|IsDiagonal _index_2 _previousindex)))))