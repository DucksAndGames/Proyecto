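; BP_Grid is an actor that builds a hexagonal tile grid for combat from its construction script.
; It snaps center and corner, then lays tiles in doubled-row coordinates, skipping alternate Y indices and scaling by data-table mesh size.
; Optional sphere traces snap tile height to the ground and take tile type from hits, including BP_GridModifier actors.
; Tiles are stored by index and forwarded to a child BP_GridVisual for display.
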(event EventBeginPlay)

(event Collision|EventActorBeginOverlap
  (params (OtherActor :type Actor%20Object%20Reference)))

(event EventTick
  (params (DeltaSeconds :type Float%20%28single-precision%29)))

(fn ConstructionScript
  (Variables|Default|SetGridVisual (.AsBP%20Grid%20Visual (Utilities|Casting|CastToBP_GridVisual (Variables|/Script/Engine.ChildActorComponent|GetChildActor (Variables|Default|GetChildActor_GridVisual)))))
  (CallFunction|SpawnGrid (Transformation|GetActorLocation) (Variables|Default|GetGridTale%20Size) (Variables|Default|GetGridTile%20Count) true))

(fn SpawnGrid
  (params (CenterLocation :type Vector) (TaleSize :type Vector) (TileCount :type Int%20Point%20Structure) (UseEnvironment :type Boolean))
  (Variables|Default|SetGridCenter%20Location CenterLocation)
  (Variables|Default|SetGridTale%20Size TaleSize)
  (Variables|Default|SetGridTile%20Count TileCount)
  (CallFunction|DestroyGrid)
  ;[1 1 1] Comment
  (bind (_center _bottomleft) (CallFunction|CalculateCenterandBottomLeft))
  (Variables|Default|SetGridCenter%20Location _center)
  (Variables|Default|SetGridBottomLeftConerLocation _bottomleft)
  (Default|InitializeGridVisual (Variables|Default|GetGridVisual) self)
  ;[1 1 1] Comment
  (for _index (range 0 (- (.x (Variables|Default|GetGridTile%20Count)) 1))
    (LocalVariables|Setx _index)
    (for _index_2 (range (Math|Integer|SelectInt 0 1 (CallFunction|IsIntEven (LocalVariables|Getx))) (- (* (.y (Variables|Default|GetGridTile%20Count)) 2) 1))
      (LocalVariables|SetY _index_2)
      (Utilities|FlowControl|Sequence
        (:then_0
          (LocalVariables|Setindex (Utilities|Struct|MakeIntPoint (LocalVariables|Getx) (LocalVariables|GetY)))
          ;[1 1 1] Comment
          (LocalVariables|SetTileTransform (Math|Transform|MakeTransform (Utilities|GetTileLocationfromGridIndex (LocalVariables|Getindex)) (Utilities|GetTileRotationfromGridIndex (LocalVariables|Getindex)) (/ (Variables|Default|GetGridTale%20Size) (.MeshSize (Utilities|Struct|BreakS_GridShapeData (Utilities|GetCurrentShapeData))))))
          (if UseEnvironment
            ;[1 1 1] Comment
            (bind (_outlocation _tiletype) (CallFunction|TraceforGround (.location (LocalVariables|GetTileTransform))))
            (CallFunction|AddGridTile (Utilities|Struct|MakeS_TileData (LocalVariables|Getindex) _tiletype (Math|Transform|MakeTransform _outlocation (.rotation (LocalVariables|GetTileTransform)) (.scale (LocalVariables|GetTileTransform)))))
            (else
              (CallFunction|AddGridTile (Utilities|Struct|MakeS_TileData (LocalVariables|Getindex) "NewEnumerator1" (LocalVariables|GetTileTransform))))))
        (:then_1
          (Math|Integer|IncrementInt _index_2))))))

(fn GetTileLocationfromGridIndex
  (params (GrinIndex :type Int%20Point%20Structure))
  (return (+ (Variables|Default|GetGridBottomLeftConerLocation) (* (Variables|Default|GetGridTale%20Size) (* GrinIndex "(X=0.750000,Y=0.500000)")))))

(fn GetTileRotationfromGridIndex
  (params (GridIndex :type Int%20Point%20Structure))
  ;[1 1 1] Only if are triangles
  (return "0, 0, 0"))

(fn GetCurrentShapeData
  (bind _returnvalue (Utilities|GetDataTableRow "/Game/Combat/Blueprints/Core/Grid/GridShapes/DT_GridShapeData.DT_GridShapeData" "Hexagon")
    (:then
      (return _returnvalue))))

(fn DestroyGrid
  (Utilities|Map|Clear (Variables|Default|GetGridTiles))
  (Default|DestroyGridVisual (Variables|Default|GetGridVisual)))

(fn CalculateCenterandBottomLeft
  (bind _gridtale_size (Variables|Default|GetGridTale%20Size))
  (LocalVariables|SetC (CallFunction|SnapVectortoVector (Variables|Default|GetGridCenter%20Location) (* (Variables|Default|GetGridTale%20Size) "1.500000,1.000000,1.000000")))
  (return (LocalVariables|GetC) (- (LocalVariables|GetC) (CallFunction|SnapVectortoVector (* (/ (Variables|Default|GetGridTile%20Count) "(X=3.000000,Y=2.000000)") (Math|Conversions|ToVector2D(Vector) _gridtale_size)) (* _gridtale_size "1.500000,1.000000,1.000000")))))

(fn TraceforGround
  (params (Location :type Vector))
  (LocalVariables|SetRadius (/ (.x (Variables|Default|GetGridTale%20Size)) 3.0))
  (bind _outhits (Collision|MultiSphereTraceByChannel (+ Location "0,0,1000.000000") (- Location "0,0,1000.000000") (LocalVariables|GetRadius) "TraceTypeQuery3" false 0 "None"))
  (if (> (Utilities|Array|Length _outhits) 0)
    (LocalVariables|SetRetType "NewEnumerator1")
    (for _array_element _outhits
      (bind _asbp_grid_modifier (Utilities|Casting|CastToBP_GridModifier (.HitActor (Collision|BreakHitResult _array_element)))
        (:then
          (LocalVariables|SetRetType (Variables|/Game/Combat/Blueprints/Core/Grid/BP_GridModifier.BP_GridModifier_C|GetType _asbp_grid_modifier)))
        (:CastFailed
          (LocalVariables|SetRetZ (Math|Float|SnapToGrid(Float) (- (.Z (Class|KismetMathLibrary|BreakVector3f (.Location (Collision|BreakHitResult _array_element)))) (LocalVariables|GetRadius)) (.z (Variables|Default|GetGridTale%20Size)))))))
    (return (Math|Vector|MakeVector (.x Location) (.y Location) (LocalVariables|GetRetZ)) (LocalVariables|GetRetType))
    (else
      (return Location "NewEnumerator0"))))

(fn AddGridTile
  (params (Data :type S%20Tile%20Data%20Structure))
  (Utilities|Map|Add (Variables|Default|GetGridTiles) (.index Data) Data)
  (Default|UpdateTileVisual (Variables|Default|GetGridVisual) Data))