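; BP_GridModifier is an editor-placed volume that marks a combat grid tile type, such as obstacle, higher movement cost or flying-only.
; Its construction script applies the hardcoded Hexagon row's mesh and flat material from DT_GridShapeData, then tints it by Type through material parameters.
; It overlaps a custom trace channel, presumably for grid detection, and is hidden in game; the event graph is empty.
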(event EventBeginPlay)

(event Collision|EventActorBeginOverlap
  (params (OtherActor :type Actor%20Object%20Reference)))

(event EventTick
  (params (DeltaSeconds :type Float%20%28single-precision%29)))

(fn ConstructionScript
  (bind _staticmesh (Variables|Default|GetStaticMesh))
  ;[1 1 1] Set volume's visual based on the shape and type
  (bind _returnvalue (Utilities|GetDataTableRow "/Game/Combat/Blueprints/Core/Grid/GridShapes/DT_GridShapeData.DT_GridShapeData" "Hexagon")
    (:then
      (Components|StaticMesh|SetStaticMesh _staticmesh (.Mesh (Utilities|Struct|BreakS_GridShapeData _returnvalue)))
      (Rendering|Material|SetMaterial (Variables|Default|GetStaticMesh) 0 (.FlatMaterial (Utilities|Struct|BreakS_GridShapeData _returnvalue)))
      (Rendering|Material|SetVectorParameterValueonMaterials _staticmesh "Color" (Math|Conversions|ToVector(LinearColor) (Utilities|Select :Index (Variables|Default|GetType) :NewEnumerator0 "" :NewEnumerator1 "(R=1.000000,G=1.000000,B=1.000000,A=1.000000)" :NewEnumerator2 "(R=1.000000,G=0.000000,B=0.000000,A=1.000000)" :NewEnumerator3 "(R=1.000000,G=0.877390,B=0.000000,A=1.000000)" :NewEnumerator4 "(R=1.000000,G=0.000000,B=0.433389,A=1.000000)" :NewEnumerator5 "(R=0.000000,G=1.000000,B=0.903017,A=1.000000)")))
      (Rendering|Material|SetScalarParameterValueonMaterials (Variables|Default|GetStaticMesh) "IsFilled" 1.0)
      (Collision|SetCollisionResponsetoChannel (Variables|Default|GetStaticMesh) "ECC_GameTraceChannel1" "ECR_Overlap")
      (Rendering|SetActorHiddenInGame true))))