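; BP_Unit is the combat unit Blueprint, whose appearance is driven by its UnitType.
; The construction script looks up default unit data for that type and applies its skeletal mesh and Animation Blueprint.
; BeginPlay runs an endless test loop that advances TestAnimIndex every few seconds and sends it to the anim instance through SetUnitAnimationStateMessage.
; The modulo wrap cycles the first five animation states, so the sixth Select option is never reached.
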(event EventBeginPlay
  (Utilities|FlowControl|Delay 3.0 :!label _label)
  (bind _output_get (Variables|Default|SetTestAnimIndex (Utilities|Select :Index (Math|Integer|%(Integer) (+ (Math|Conversions|ToInteger(Byte) (Variables|Default|GetTestAnimIndex)) 1) 5) :Option%200 "NewEnumerator0" :Option%201 "NewEnumerator1" :Option%202 "NewEnumerator2" :Option%203 "NewEnumerator3" :Option%204 "NewEnumerator4" :Option%205 "NewEnumerator5")))
  (Class|BPIUnitAnimation|SetUnitAnimationState(Message) (Components|SkeletalMesh|GetAnimInstance (Variables|Default|GetSkeletalMesh)) _output_get)
  (goto _label))

(fn ConstructionScript
  (bind _skeletalmesh (Variables|Default|GetSkeletalMesh))
  (bind _unitdata (CallFunction|GetDefaultUnitDatafromUnitType (Variables|Default|GetUnitType)))
  (Class|SkinnedMeshComponent|SetSkeletalMesh _skeletalmesh (.Mesh (Utilities|Struct|BreakS_UnitData_Assests (.Assets (Utilities|Struct|BreakS_UnitData _unitdata)))) true)
  (Class|SkeletalMeshComponent|SetAnimClass _skeletalmesh (.AnimBP (Utilities|Struct|BreakS_UnitData_Assests (.Assets (Utilities|Struct|BreakS_UnitData _unitdata))))))