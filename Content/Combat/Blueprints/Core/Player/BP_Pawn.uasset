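; BP_Pawn is the player's camera pawn for the combat game, with smoothed panning, zooming and stepped rotation.
; Axis inputs shift a desired location along the pawn's forward and right vectors and adjust a clamped spring arm length, while rotate actions add fixed yaw steps.
; Tick interpolates location, rotation and arm length toward those targets, moving without sweep so collision does not block it.
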(event EventTick
  (params (DeltaSeconds :type Float%20%28single-precision%29))
  (bind _springarm (Variables|Default|GetSpringArm))
  (Variables|/Script/Engine.SpringArmComponent|SetTargetArmLength _springarm (Math|Interpolation|FInterpTo (Variables|/Script/Engine.SpringArmComponent|GetTargetArmLength _springarm) (Variables|Default|GetZoom_Desired) DeltaSeconds (Variables|Default|GetZoomInterpSpeed)))
  (Transformation|SetActorLocation (Math|Interpolation|VInterpTo (Transformation|GetActorLocation) (Variables|Default|GetLocation_Desired) DeltaSeconds (Variables|Default|GetLocationInterpSpeed)) false false)
  (Transformation|SetActorRotation (Math|Interpolation|RInterpTo (Transformation|GetActorRotation) (Variables|Default|GetRotation_Desired) DeltaSeconds (Variables|Default|GetRotationInterpSpeed))))

(event EventBeginPlay
  (Variables|Default|SetLocation_Desired (Transformation|GetActorLocation))
  (Variables|Default|SetZoom_Desired (Variables|/Script/Engine.SpringArmComponent|GetTargetArmLength (Variables|Default|GetSpringArm)))
  (Variables|Default|SetRotation_Desired (Transformation|GetActorRotation)))

(event Input|ActionEvents|InputActionAction_Rotate_Right
  (params (Key :type Key%20Structure :default "None"))
  (:Pressed
    (Variables|Default|SetRotation_Desired (Math|Rotator|CombineRotators (Variables|Default|GetRotation_Desired) (Math|Rotator|MakeRotator 0.0 0.0 (Variables|Default|GetRotationSpeed))))))

(event Input|ActionEvents|InputActionAction_Rotate_Left
  (params (Key :type Key%20Structure :default "None"))
  (:Pressed
    (Variables|Default|SetRotation_Desired (Math|Rotator|CombineRotators (Variables|Default|GetRotation_Desired) (Math|Rotator|MakeRotator 0.0 0.0 (- 0.0 (Variables|Default|GetRotationSpeed)))))))

(event Input|AxisEvents|InputAxisInputAxis_Zoom
  (params (AxisValue :type Float%20%28single-precision%29))
  (Variables|Default|SetZoom_Desired (Math|Float|Clamp(Float) (+ (Variables|Default|GetZoom_Desired) (* AxisValue (* (Variables|Default|GetZoomSpeed) -1.0))) (Variables|Default|GetZoomMin) (Variables|Default|GetZoomMax))))

(event Input|AxisEvents|InputAxisInputAxis_Forward
  (params (AxisValue :type Float%20%28single-precision%29))
  (Variables|Default|SetLocation_Desired (+ (Variables|Default|GetLocation_Desired) (* (Transformation|GetActorForwardVector) (* AxisValue (Variables|Default|GetLocationSpeed))))))

(event Input|AxisEvents|InputAxisInputAxis_Right
  (params (AxisValue :type Float%20%28single-precision%29))
  (Variables|Default|SetLocation_Desired (+ (Variables|Default|GetLocation_Desired) (* (Transformation|GetActorRightVector) (* AxisValue (Variables|Default|GetLocationSpeed))))))

(fn ConstructionScript)